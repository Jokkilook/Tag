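; Enemy pawn that uses PawnSensing to drive Chase and Search states through AI Blackboard keys.
; Seeing the player stores actor and location and starts Chase; hearing noise stores its location and switches to Search.
; Tick drops Chase to Search once the player goes unseen beyond a delay, tracked with a mirrored local state.
; The node assigning the Blackboard reference is unconnected, so this graph never sets it.
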(event `self.ReceiveBeginPlay`
  (bind _returnvalue (`self.GetController`))
  (bind _asbp_enemy_aicontroller (cast `/Game/Enemy/BP_EnemyAIController` _returnvalue)))

(event `self.ReceiveTick`
  (params (DeltaSeconds :type "Float (single-precision)"))
  (bind _returnvalue (`KismetSystemLibrary.GetGameTimeInSeconds`))
  (if (`|EnumEquality` (`self.CurrentState`) (`self.Value_Chase`))
    (set `self.NowTime` _returnvalue)
    (if (> (`self.NowTime`) (+ (`self.LastSeenTime`) (`self.ChaseLostDelay`)))
      (`BlackboardComponent.SetValueAsEnum` (`self.BlackboardRef`) (`self.Key_State`) (`self.Value_Search`))
      (set `self.CurrentState` (`self.Value_Search`))
      (set `self.LastSeenTime` (`self.NowTime`)))))

(event `self.PawnSensing.OnSeePawn`
  (params (Pawn :type "Pawn Object Reference"))
  (bind _blackboardref (`self.BlackboardRef`))
  (bind _asbp_player (cast `/Game/Enemy/BP_Player` Pawn))
  (`BlackboardComponent.SetValueAsObject` _blackboardref (`self.Key_PlayerActor`) _asbp_player)
  (`BlackboardComponent.SetValueAsVector` _blackboardref (`self.Key_LastSeenLocation`) (`self.K2_GetActorLocation` _asbp_player))
  (`BlackboardComponent.SetValueAsEnum` _blackboardref (`self.Key_State`) (`self.Value_Chase`))
  (bind _returnvalue (`KismetSystemLibrary.GetGameTimeInSeconds`))
  (set `self.LastSeenTime` _returnvalue)
  (set `self.CurrentState` (`self.Value_Chase`)))

(event `self.PawnSensing.OnHearNoise`
  (params (Instigator :type "Pawn Object Reference") (Location :type "Vector Structure (by ref)") (Volume :type "Float (single-precision)"))
  (`BlackboardComponent.SetValueAsVector` (`self.BlackboardRef`) (`self.Key_LastHeardLocation`) Location)
  (`BlackboardComponent.SetValueAsEnum` (`self.BlackboardRef`) (`self.Key_State`) (`self.Value_Search`))
  (bind _returnvalue (`KismetSystemLibrary.GetGameTimeInSeconds`))
  (set `self.LastSeenTime` _returnvalue)
  (set `self.CurrentState` (`self.Value_Search`)))

(fn `UserConstructionScript`)