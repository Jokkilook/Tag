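; First-person player character Blueprint that adds the HUD, plays footsteps and lets the player interact with objects in view.
; Each tick, a visibility line trace from the camera caches any hit actor implementing BPI_Interaction as the target and sets an interaction flag.
; The interact input sends InteractionMessage to that target without checking the flag.
; Move input starts and stops a looping timer that plays footstep sounds at the character's location.
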(event `EnhancedInput|/Game/FirstPerson/Input/Actions/IA_Move`
  (params (ActionValue :type "Vector2D Structure") (ElapsedSeconds :type "Float (double-precision)") (TriggeredSeconds :type "Float (double-precision)") (InputAction :type "InputAction Object Reference" :default "/Game/FirstPerson/Input/Actions/IA_Move.IA_Move"))
  (:`Started`
    (`self.StartFootStep`))
  (:`Completed`
    (`self.StopFootStep`)))

(event `self.ReceiveBeginPlay`
  (bind _returnvalue (`GameplayStatics.GetPlayerController` 0))
  (bind _returnvalue_2 (`|CreateWidget` "/Game/Blueprints/WBP_HUD.WBP_HUD_C" null self))
  (`WidgetBlueprintLibrary.SetInputMode_GameOnly` _returnvalue)
  (set `PlayerController.bShowMouseCursor` false _returnvalue)
  (`UserWidget.AddToViewport` _returnvalue_2 0))

(event `self.ReceiveTick`
  (params (DeltaSeconds :type "Float (single-precision)"))
  (bind _firstpersoncameracomponent (`self.FirstPersonCameraComponent`))
  (bind _returnvalue (`SceneComponent.K2_GetComponentLocation` _firstpersoncameracomponent))
  (bind (_outhit _returnvalue_2) (`KismetSystemLibrary.LineTraceSingle` _returnvalue (+ _returnvalue (* (`SceneComponent.GetForwardVector` _firstpersoncameracomponent) 500.0)) "TraceTypeQuery1"))
  (if _returnvalue_2
    (bind (_bblockinghit _binitialoverlap _time _distance _location _impactpoint _normal _impactnormal _physmat _hitactor) (`GameplayStatics.BreakHitResult` _outhit))
    (if (`KismetSystemLibrary.DoesImplementInterface` _hitactor "/Game/Blueprints/BPI_Interaction.BPI_Interaction_C")
      (set `self.TargetActor` _hitactor)
      (set `self.CanInteraction` true)
      (else
        (set `self.TargetActor` null)
        (set `self.CanInteraction` false)))
    (else
      (set `self.TargetActor` null)
      (set `self.CanInteraction` false))))

(event `EnhancedInput|/Game/HYH/Inputs/IA_Interaction`
  (params (ActionValue :type Boolean) (ElapsedSeconds :type "Float (double-precision)") (TriggeredSeconds :type "Float (double-precision)") (InputAction :type "InputAction Object Reference" :default "/Game/HYH/Inputs/IA_Interaction.IA_Interaction"))
  (:`Started`
    (message `/Game/Blueprints/BPI_Interaction.Interaction` (`self.TargetActor`) self)))

(fn `PlayFootStep`
  (`GameplayStatics.PlaySoundAtLocation` "/Game/FootstepsMiniPack/SC_Foot.SC_Foot" (`self.K2_GetActorLocation`) (struct) 1.0 1.0 0.0 null null null null))

(fn `StartFootStep`
  (`KismetSystemLibrary.K2_SetTimer` null "PlayFootStep" 0.4 true))

(fn `StopFootStep`
  (`KismetSystemLibrary.K2_ClearTimer` null "PlayFootStep"))

(fn `UserConstructionScript`)