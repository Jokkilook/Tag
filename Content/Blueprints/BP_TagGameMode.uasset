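; Game mode for a tag game that, on BeginPlay, scatters key items and shows a brief "Find exit door." message through WBP_LockInfo.
; SetGameItem makes one pass over all BP_SpawnPoint actors, giving each a 20% chance of selection, up to three.
; BP_ItemA, B and C spawn at the chosen points in selection order, so fewer items appear if fewer points are picked.
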(event `self.ReceiveBeginPlay`
  (`self.SetGameItem`)
  (bind _returnvalue (`|CreateWidget` "/Game/Widgets/WBP_LockInfo.WBP_LockInfo_C" null "Find exit door." 3.0))
  (`UserWidget.AddToViewport` _returnvalue 0))

(fn `SetGameItem`
  (locals (TargetPoints :type "Array of /Game/Blueprints/BP_SpawnPoint Object Reference"))
  (bind _targetpoints (`local.TargetPoints`))
  (bind _outactors (`GameplayStatics.GetAllActorsOfClass` "/Game/Blueprints/BP_SpawnPoint.BP_SpawnPoint_C"))
  (for _array_element _outactors
    (if (< (`KismetMathLibrary.RandomFloat`) 0.2)
      (if (>= (`KismetArrayLibrary.Array_Length` _targetpoints) 3)
        (break)
        (elif (not (`KismetArrayLibrary.Array_Contains` _targetpoints _array_element))
          (`KismetArrayLibrary.Array_Add` (`local.TargetPoints`) _array_element)))))
  (for (_array_element_2 _array_index) (`local.TargetPoints`)
    (switch `int` _array_index
      (:`0`
        (bind _returnvalue (`self.GetTransform` _array_element_2))
        (`|SpawnActorFromClass` "/Game/Blueprints/BP_ItemA.BP_ItemA_C" _returnvalue "AdjustIfPossibleButAlwaysSpawn" "MultiplyWithRoot" null null))
      (:`1`
        (`|SpawnActorFromClass` "/Game/Blueprints/BP_ItemB.BP_ItemB_C" _returnvalue "AdjustIfPossibleButAlwaysSpawn" "MultiplyWithRoot" null null))
      (:`2`
        (`|SpawnActorFromClass` "/Game/Blueprints/BP_ItemC.BP_ItemC_C" _returnvalue "AdjustIfPossibleButAlwaysSpawn" "MultiplyWithRoot" null null)))))

(fn `UserConstructionScript`)