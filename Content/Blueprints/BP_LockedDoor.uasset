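; Locked door actor that swings open when an interactor carrying all three required keys uses it.
; Interaction calls CheckHasKey, which looks up the interactor's BPC_InventoryComponent and requires items A, B and C in its Items.
; On success, Open plays the OpenDoor timeline, whose update lerps the Door's relative yaw a quarter turn.
; Close reverses that timeline, though nothing in this Blueprint calls it.
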(event `/Game/Blueprints/BPI_Interaction.Interaction`
  (params (Interactor :type "Actor Object Reference"))
  (bind _ispass (`self.CheckHasKey` Interactor))
  (if _ispass
    (`self.Open`)))

(event `Open`
  (bind (_direction _delta) (`Timeline|OpenDoor` :!label _label)
    (:`Update`
      (`SceneComponent.K2_SetRelativeRotation` (`self.Door`) (`KismetMathLibrary.MakeRotator` 0.0 0.0 (`KismetMathLibrary.Lerp` 0.0 -90.0 _delta)) false false))))

(event `Close`
  (goto _label :!via `Reverse`))

(fn `CheckHasKey`
  (params (Checker :type "Actor Object Reference"))
  (returns (IsPass :type Boolean))
  (locals (B :type Boolean) (A :type Boolean) (C :type Boolean))
  (bind _items (`/Game/Components/BPC_InventoryComponent.Items` (`self.GetComponentByClass` Checker "/Game/Components/BPC_InventoryComponent.BPC_InventoryComponent_C")))
  (`|ExecutionSequence`
    (:`then_0`
      (if (`KismetArrayLibrary.Array_Contains` _items "A")
        (set `local.A` true)))
    (:`then_1`
      (if (`KismetArrayLibrary.Array_Contains` _items "B")
        (set `local.B` true)))
    (:`then_2`
      (if (`KismetArrayLibrary.Array_Contains` _items "C")
        (set `local.C` true)))
    (:`then_3`
      (return (and (`local.A`) (`local.B`) (`local.C`))))))

(fn `UserConstructionScript`)